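; BlueBirdBP is the blue bird, whose ability splits it into three by spawning two more copies of itself.
; The BlueBirdAbility event spawns one copy above and one below the bird, offset by VerticalOffset on Z.
; Each copy's BirdMesh receives the original's current velocity as a velocity-change impulse, so the copies launch with the same motion regardless of mass.
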(event Custom|BlueBirdAbility
  (bind _returnvalue (Transformation|GetActorLocation))
  (bind _returnvalue_2 (Transformation|GetActorLocation))
  (bind _returnvalue_3 (Transformation|GetVelocity))
  (bind _returnvalue_4 (Game|SpawnActorfromClass "BlueBirdBP_C" (Math|Conversions|ToTransform(Vector) (Math|Vector|MakeVector (.x _returnvalue_2) (.y _returnvalue_2) (+ (.z _returnvalue_2) (Variables|Default|GetVertical%20Offset)))) "Undefined" "MultiplyWithRoot" 0 0))
  (Physics|AddImpulse (Variables|/Script/AngryBirds.Bird|GetBirdMesh _returnvalue_4) _returnvalue_3 "None" true)
  (bind _returnvalue_5 (Game|SpawnActorfromClass "BlueBirdBP_C" (Math|Conversions|ToTransform(Vector) (Math|Vector|MakeVector (.x _returnvalue) (.y _returnvalue) (- (.z _returnvalue) (Variables|Default|GetVertical%20Offset)))) "Undefined" "MultiplyWithRoot" 0 0))
  (Physics|AddImpulse (Variables|/Script/AngryBirds.Bird|GetBirdMesh _returnvalue_5) _returnvalue_3 "None" true))

(fn ConstructionScript
  (|CallParentFunction))