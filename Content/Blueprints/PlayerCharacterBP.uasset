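; Slingshot player character for an Angry Birds-style game that aims and launches red, blue or yellow birds.
; Touch drag sets launch velocity, and Tick spawns indicator actors along the predicted projectile path.
; Release spawns the key-selected bird at LaunchPoint with an impulse, unless that type's bird still exists.
; Space triggers its ability, V toggles the bird view, and Tick reactivates PlayerCamera when no selected bird exists.
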(event EventBeginPlay
  (bind _returnvalue (Game|GetPlayerController 0))
  (Input|SetInputModeGameOnly _returnvalue false)
  (Variables|/Script/Engine.PlayerController|SetbShowMouseCursor _returnvalue true))

(event EventTick
  (params (DeltaSeconds :type Float%20%28single-precision%29))
  (Utilities|FlowControl|Sequence
    (:then_0
      (if (Variables|Default|GetTouchPressed)
        (bind _returnvalue (Class|WidgetLayoutLibrary|GetMousePositiononViewport))
        (bind _output_get (Variables|Default|SetBirdlaunchForce (Math|Vector|MakeVector 0.0 (* (.x (- _returnvalue (Variables|Default|GetMousePosition))) -2.0) (.y (- _returnvalue (Variables|Default|GetMousePosition))))))
        (bind _outpathpositions (Class|GameplayStatics|BlueprintPredictProjectilePathbyTraceChannel (Transformation|GetWorldLocation (Variables|Default|GetLaunchPoint)) _output_get true 5.0 "ECC_WorldDynamic" false 0 "None" 1.0 2e+01 1.0))
        (for _array_element _outpathpositions
          (Game|SpawnActorfromClass "/Game/Blueprints/PredictionIndicatorBp.PredictionIndicatorBp_C" (Math|Conversions|ToTransform(Vector) _array_element) "Undefined" "MultiplyWithRoot" 0 0))))
    (:then_1
      (Utilities|IsValid (Utilities|Select :Index (Variables|Default|GetBirdType) :Option%200 (Variables|Default|GetRedBird) :Option%201 (Variables|Default|GetBlueBird) :Option%202 (Variables|Default|GetYellowBird))
        (:Is%20Not%20Valid
          (Components|Activation|SetActive (Variables|Default|GetPlayerCamera) true false))))))

(event Input|KeyboardEvents|V
  (params (Key :type Key%20Structure :default "None"))
  (bind _playercamera (Variables|Default|GetPlayerCamera))
  (:Pressed
    (Utilities|FlowControl|FlipFlop
      (:A
        (if (Components|Activation|IsActive _playercamera)
          (Utilities|IsValid (Utilities|Select :Index (Variables|Default|GetBirdType) :Option%200 (Variables|Default|GetRedBird) :Option%201 (Variables|Default|GetBlueBird) :Option%202 (Variables|Default|GetYellowBird))
            (:Is%20Valid
              (Game|Player|SetViewTargetwithBlend (Game|GetPlayerController 0) (Utilities|Select :Index (Variables|Default|GetBirdType) :Option%200 (Variables|Default|GetRedBird) :Option%201 (Variables|Default|GetBlueBird) :Option%202 (Variables|Default|GetYellowBird)) 0.5 "VTBlend_Cubic" 0.0 false)
              (Components|Activation|SetActive (Variables|Default|GetPlayerCamera) false false)))
          (else
            (Components|Activation|SetActive _playercamera true false :!label _label))))
      (:B
        (goto _label)))))

(event Input|KeyboardEvents|2
  (params (Key :type Key%20Structure :default "None"))
  (:Pressed
    (Variables|Default|SetBirdType 1)))

(event Input|KeyboardEvents|1
  (params (Key :type Key%20Structure :default "None"))
  (:Pressed
    (Variables|Default|SetBirdType 0)))

(event Input|KeyboardEvents|3
  (params (Key :type Key%20Structure :default "None"))
  (:Pressed
    (Variables|Default|SetBirdType 2)))

(event Input|KeyboardEvents|SpaceBar
  (params (Key :type Key%20Structure :default "None"))
  (:Released
    (Utilities|IsValid (Utilities|Select :Index (Variables|Default|GetBirdType) :Option%200 (Variables|Default|GetRedBird) :Option%201 (Variables|Default|GetBlueBird) :Option%202 (Variables|Default|GetYellowBird))
      (:Is%20Valid
        (switch int (Variables|Default|GetBirdType)
          (:0
            (Default|RedBirdAbility (Variables|Default|GetRedBird)))
          (:1
            (Default|BlueBirdAbility (Variables|Default|GetBlueBird)))
          (:2
            (Default|YellowBirdAbility (Variables|Default|GetYellowBird))))))))

(event Input|TouchEvents|InputTouch
  (params (Location :type Vector) (FingerIndex :type ETouchIndex%20Enum))
  (bind _launchpoint (Variables|Default|GetLaunchPoint))
  (bind _returnvalue (Transformation|GetWorldLocation _launchpoint))
  (bind _returnvalue_2 (Math|Conversions|ToTransform(Vector) _returnvalue))
  (:Pressed
    (Variables|Default|SetTouchPressed true)
    (bind _returnvalue_3 (Class|WidgetLayoutLibrary|GetMousePositiononViewport))
    (Variables|Default|SetMousePosition _returnvalue_3))
  (:Released
    (Variables|Default|SetTouchPressed false)
    (Utilities|IsValid (Utilities|Select :Index (Variables|Default|GetBirdType) :Option%200 (Variables|Default|GetRedBird) :Option%201 (Variables|Default|GetBlueBird) :Option%202 (Variables|Default|GetYellowBird))
      (:Is%20Not%20Valid
        (switch int (Variables|Default|GetBirdType)
          (:0
            (bind _returnvalue_4 (Game|SpawnActorfromClass "/Game/Blueprints/Birds/RedBirdBP.RedBirdBP_C" _returnvalue_2 "Undefined" "MultiplyWithRoot" 0 0))
            (bind _output_get (Variables|Default|SetRedBird _returnvalue_4))
            (Physics|AddImpulse (Variables|/Script/AngryBirds.Bird|GetBirdMesh _output_get) (Variables|Default|GetBirdlaunchForce) "None" true))
          (:1
            (bind _returnvalue_5 (Game|SpawnActorfromClass "/Game/Blueprints/Birds/BlueBirdBP.BlueBirdBP_C" _returnvalue_2 "Undefined" "MultiplyWithRoot" 0 0))
            (bind _output_get_2 (Variables|Default|SetBlueBird _returnvalue_5))
            (Physics|AddImpulse (Variables|/Script/AngryBirds.Bird|GetBirdMesh _output_get_2) (Variables|Default|GetBirdlaunchForce) "None" true))
          (:2
            (bind _returnvalue_6 (Game|SpawnActorfromClass "/Game/Blueprints/Birds/YellowBirdBP.YellowBirdBP_C" _returnvalue_2 "Undefined" "MultiplyWithRoot" 0 0))
            (bind _output_get_3 (Variables|Default|SetYellowBird _returnvalue_6))
            (Physics|AddImpulse (Variables|/Script/AngryBirds.Bird|GetBirdMesh _output_get_3) (Variables|Default|GetBirdlaunchForce) "None" true)))))))

(fn ConstructionScript)